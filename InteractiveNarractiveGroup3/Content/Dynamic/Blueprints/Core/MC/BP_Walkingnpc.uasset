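; BP_Walkingnpc is a wandering NPC pawn that walks endlessly between random reachable points on the navmesh.
; On BeginPlay it picks a random skeletal mesh from its Meshes array using a hardcoded index range, then starts moving.
; AI MoveTo targets a point within a very large radius of the capsule, and both success and failure print the result and call Reset to choose another destination.
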(event Custom|Reset
  (bind _movementresult (AI|AIMoveTo self (.RandomLocation (AI|Navigation|GetRandomReachablePointinRadius (Transformation|GetWorldLocation (Variables|Collision|GetCapsuleComponent)) 1e+05 0 0)) 0 5.0 false)
    (:OnSuccess
      (Development|PrintString (Utilities|String|EnumtoString _movementresult)))
    (:OnFail
      (Development|PrintString (Utilities|String|EnumtoString _movementresult))))
  (CallFunction|Reset))

(event EventBeginPlay
  (Components|SkeletalMesh|SetSkeletalMeshAsset (Variables|Character|GetMesh) (Utilities|Array|Get(acopy) (Variables|Default|GetMeshes) (Math|Random|RandomIntegerinRange 0 45)))
  (bind _movementresult (AI|AIMoveTo self (.RandomLocation (AI|Navigation|GetRandomReachablePointinRadius (Transformation|GetWorldLocation (Variables|Collision|GetCapsuleComponent)) 1e+05 0 0)) 0 5.0 false)
    (:OnSuccess
      (Development|PrintString (Utilities|String|EnumtoString _movementresult)))
    (:OnFail
      (Development|PrintString (Utilities|String|EnumtoString _movementresult))))
  (CallFunction|Reset))

(fn ConstructionScript)