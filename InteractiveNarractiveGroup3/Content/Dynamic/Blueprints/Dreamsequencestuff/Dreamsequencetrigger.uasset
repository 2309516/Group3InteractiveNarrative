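; Interactable trigger that sends the player into the dream sequence.
; On Interact it calls CutsceneStarter, shows a Blink widget and teleports the player character to a hardcoded world location behind it.
; After a short delay it removes the widget and unhides the StaticMesh component on BP_FirstPersonCharacter.
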(event EventBeginPlay)

(event Collision|EventActorBeginOverlap
  (params (OtherActor :type Actor%20Object%20Reference)))

(event EventTick
  (params (DeltaSeconds :type Float%20%28single-precision%29)))

(event EventInteract
  (Default|CallCutsceneStarter)
  (bind _returnvalue (UserInterface|CreateWidget "/Game/Dynamic/Blueprints/Dreamsequencestuff/Blink.Blink_C" (Game|GetPlayerController 0)))
  (UserInterface|Viewport|AddtoViewport _returnvalue 0)
  (Transformation|Teleport (Game|GetPlayerCharacter 0) "38220.000000,-62560.000000,0.000000" "0, 0, 0")
  (Utilities|FlowControl|Delay 1.0)
  (Widget|RemovefromParent _returnvalue)
  (bind _asbp_first_person_character (Utilities|Casting|CastToBP_FirstPersonCharacter (Game|GetPlayerCharacter 0)))
  (Development|SetHiddeninGame (Variables|/Game/Dynamic/Blueprints/Core/MC/BP_FirstPersonCharacter.BP_FirstPersonCharacter_C|GetStaticMesh _asbp_first_person_character) false false))

(fn ConstructionScript)